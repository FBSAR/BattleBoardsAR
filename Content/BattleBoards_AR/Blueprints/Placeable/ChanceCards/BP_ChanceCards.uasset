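; BP_ChanceCards is a placeable chance card actor for the AR battle board game, currently with no working behavior.
; BeginPlay, FlipCard and the construction script are empty.
; Unconnected nodes sketch a flip animation: find the BP_CardPath actor, then use the CardFlip timeline to move and rotate the card along its spline.
; That logic samples location in world space but rotation in local space, and never runs.
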(event `self.ReceiveBeginPlay`)

(event `FlipCard`)

(fn `UserConstructionScript`)