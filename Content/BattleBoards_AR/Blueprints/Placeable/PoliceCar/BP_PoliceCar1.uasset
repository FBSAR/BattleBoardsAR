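; BP_PoliceCar1 is a placeable police car that stays hidden until MoveObject sends it along the spline of the BP_Track found at BeginPlay.
; MoveObject shows the car, attaches a siren sound and plays a timeline, rate-scaled to a set travel time, that sets its transform by spline distance.
; A self-looping FlipFlop with short delays alternates red and blue lights until, shortly after arrival, the car mesh hides and flashing stops.
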(event `self.ReceiveBeginPlay`
  (bind _returnvalue (`GameplayStatics.GetActorOfClass` "/Game/BattleBoards_AR/Blueprints/Placeable/PoliceCar/BP_Track.BP_Track_C"))
  (set `self.Spline Ref` _returnvalue)
  (`SceneComponent.SetVisibility` (`self.DefaultSceneRoot`) false true))

(event `Move Object`
  (bind _spline (`/Game/BattleBoards_AR/Blueprints/Placeable/PoliceCar/BP_Track.Spline` (`self.Spline Ref`)))
  (set `self.IsFlashing` true)
  (`SceneComponent.SetVisibility` (`self.DefaultSceneRoot`) true true)
  (`self.StartFlashingLIghts`)
  (`GameplayStatics.SpawnSoundAttached` "/Game/BattleBoards_AR/Blueprints/Placeable/PoliceCar/Siren_sounds.Siren_sounds" (`self.DefaultSceneRoot`) "None" (0.0 0.0 0.0) (struct) "KeepRelativeOffset" false 0.09 1.0 0.0 null null)
  (`TimelineComponent.SetPlayRate` (`self.Move Object T`) (/ 1.0 (`self.Time To Complete (In Seconds)`)))
  (bind (_direction _move_track) (`Timeline|Move Object T`)
    (:`Update`
      (bind _returnvalue (`KismetMathLibrary.Lerp` 0.0 (`SplineComponent.GetSplineLength` (`/Game/BattleBoards_AR/Blueprints/Placeable/PoliceCar/BP_Track.Spline` (`self.Spline Ref`))) _move_track))
      (`self.K2_SetActorTransform` (`KismetMathLibrary.MakeTransform` (`SplineComponent.GetLocationAtDistanceAlongSpline` _spline _returnvalue "World") (`SplineComponent.GetRotationAtDistanceAlongSpline` _spline _returnvalue "Local"))))
    (:`Finished`
      (`KismetSystemLibrary.Delay` 2.0)
      (`SceneComponent.SetVisibility` (`self.Car`) false true)
      (set `self.IsFlashing` false))))

(event `StartFlashingLIghts`
  (if (`self.IsFlashing`) :!label _label
    (`/Engine/EditorBlueprintResources/StandardMacros.FlipFlop`
      (:`A`
        (`SceneComponent.SetVisibility` (`self.RedLight`) true false)
        (`KismetSystemLibrary.Delay` 0.1)
        (`SceneComponent.SetVisibility` (`self.RedLight`) false false)
        (goto _label))
      (:`B`
        (`SceneComponent.SetVisibility` (`self.BlueLight`) true false)
        (`KismetSystemLibrary.Delay` 0.1)
        (`SceneComponent.SetVisibility` (`self.BlueLight`) false false)
        (goto _label)))))

(fn `UserConstructionScript`)