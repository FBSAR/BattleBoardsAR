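; Placeable AR battle board actor, mostly a stub in its current state.
; On BeginPlay it caches the AR pawn from the Monopoly Classic game mode and creates a dynamic material with a grey texture.
; CalculateTargetPosition stores the BP_Assassin's location and switches on Up, with no movement logic attached.
; The Tick interaction check is empty, and leftover visual-init and hit-die nodes are disconnected.
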(event `self.ReceiveTick`
  (params (DeltaSeconds :type "Float (single-precision)"))
  ;[1 1 1] Update HUD interaction
  (if (`self.IsInteracting`)
    _))

(event `self.ReceiveBeginPlay`
  (`|ExecutionSequence`
    (:`then_0`
      ;[1 1 1] Get Reference to AR_Pawn
      (bind _asbp_monopoly_classic_game_mode (cast `/Game/BattleBoards_AR/Blueprints/GameFramework/BP_MonopolyClassicGameMode` (`GameplayStatics.GetGameMode`)))
      (set `self.BP ARPawn` (`/Game/BattleBoards_AR/Blueprints/GameFramework/BP_MonopolyClassicGameMode.BP_ARPawn` _asbp_monopoly_classic_game_mode)))
    (:`then_2`
      ;[1 1 1] Init Axis
      (bind _returnvalue (`KismetMaterialLibrary.CreateDynamicMaterialInstance` null))
      (`MaterialInstanceDynamic.SetTextureParameterValue` _returnvalue "Texture" "/Engine/ArtTools/RenderToTexture/Textures/127grey.127grey"))))

(event `CalculateTargetPosition`
  (bind _returnvalue (`GameplayStatics.GetActorOfClass` "/Game/BattleBoards_AR/Meshes/Armies/BP_Assassin.BP_Assassin_C"))
  (set `self.CurrentPosition` (`self.K2_GetActorLocation` _returnvalue))
  (switch `/Game/BattleBoards_AR/Blueprints/UI/EDirection` "NewEnumerator0"))

(fn `UserConstructionScript`)