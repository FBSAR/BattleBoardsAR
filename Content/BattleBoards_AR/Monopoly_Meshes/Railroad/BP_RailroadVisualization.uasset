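; BP_RailroadVisualization is a Monopoly railroad visual for the AR board game, showing an animated passing train.
; It starts hidden on BeginPlay until StartSequence reveals the whole component hierarchy, plays the TrainSequence level sequence and plays a 2D train pass-by sound.
; Reset jumps the sequence playback position by time and hides everything again.
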(event `self.ReceiveBeginPlay`
  (`SceneComponent.SetVisibility` (`self.DefaultSceneRoot`) false true))

(fn `Reset`
  (`MovieSceneSequencePlayer.SetPlaybackPosition` (`ActorSequenceComponent.SequencePlayer` (`self.TrainSequence`)) (make `MovieSceneSequencePlaybackParams` (struct :`FrameNumber` (struct)) 0.0 "" "Time" "Jump"))
  (`SceneComponent.SetVisibility` (`self.DefaultSceneRoot`) false true))

(fn `StartSequence`
  (`SceneComponent.SetVisibility` (`self.DefaultSceneRoot`) true true)
  (`MovieSceneSequencePlayer.Play` (`ActorSequenceComponent.SequencePlayer` (`self.TrainSequence`)))
  (`GameplayStatics.PlaySound2D` "/Game/BattleBoards_AR/Monopoly_Meshes/Railroad/Train/train-pass-by-02.train-pass-by-02" 1.0 1.0 0.0 null null))

(fn `UserConstructionScript`)